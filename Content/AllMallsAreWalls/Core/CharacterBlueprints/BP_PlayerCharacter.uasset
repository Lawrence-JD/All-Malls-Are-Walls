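; Player character for a mall-themed game with a purse melee attack and three unlockable, cooldown-gated abilities: drink grenade, shopping-cart ride that launches a cart on release, and hitscan shot.
; The Abilities array doubles as health: each hit removes the first ability, and a hit with none left sets AmDead.
; Attached 3D icon actors show held abilities and cooldowns, while ability count drives a retro post-process overlay layered with cel shading.
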(event EventTick
  (params (DeltaSeconds :type Float%20%28single-precision%29))
  (Variables|Default|Setdrink%20cooldown (- (Variables|Default|Getdrink%20cooldown) DeltaSeconds))
  (Variables|Default|Setprojectile%20cooldown (- (Variables|Default|Getprojectile%20cooldown) DeltaSeconds))
  (Variables|Default|Setcart%20cooldown (- (Variables|Default|Getcart%20cooldown) DeltaSeconds))
  (CallFunction|UpdateTransparenctUI (Variables|Default|Getdrink%20cooldown) (Variables|Default|Getprojectile%20cooldown) (Variables|Default|Getcart%20cooldown))
  (if (< (Variables|Default|Getdrink%20cooldown) 0.0)
    (Variables|Default|Setdrink%20cooldown 0.0)
    (if (< (Variables|Default|Getprojectile%20cooldown) 0.0)
      (Variables|Default|Setprojectile%20cooldown 0.0)
      (if (< (Variables|Default|Getcart%20cooldown) 0.0)
        (Variables|Default|Setcart%20cooldown 0.0)))))

(event EventBeginPlay
  (bind _ui_scene_node (Variables|Default|GetUI_Scene_Node))
  (bind _ui_scene_node_2 (Variables|Default|GetUI_Scene_Node))
  (bind _ui_purse (Variables|Default|GetUI_Purse))
  (bind _ui_left_scene (Variables|Default|GetUI_Left_Scene))
  (bind _returnvalue (Transformation|GetWorldLocation _ui_scene_node))
  (bind _returnvalue_2 (Transformation|GetWorldLocation _ui_scene_node_2))
  (Utilities|FlowControl|Sequence
    (:then_0
      (bind _returnvalue_3 (Game|SpawnActorfromClass "/Game/AllMallsAreWalls/Core/CharacterBlueprints/Rotators/Hand_Bag.Hand_Bag_C" (Math|Transform|MakeTransform (Transformation|GetWorldLocation _ui_purse) (Transformation|GetWorldRotation _ui_purse) (Math|Vector|MakeVector 0.0 (Variables|Default|GetPurse_Scale) 0.0)) "AlwaysSpawn" 0 0))
      (Transformation|AttachComponentToComponent _returnvalue_3 (Variables|Default|GetUI_Purse) "None" "SnapToTarget" "KeepRelative" "SnapToTarget" false)
      (Variables|Default|SetLeft_UI (Math|Transform|MakeTransform (Transformation|GetWorldLocation _ui_left_scene) (Transformation|GetWorldRotation _ui_left_scene) "0.250000,0.250000,0.250000"))
      (Variables|Default|SetMiddle_UI (Math|Transform|MakeTransform (Math|Vector|MakeVector (.x _returnvalue_2) (- (.y _returnvalue_2) 0.0) (.z _returnvalue_2)) (Transformation|GetWorldRotation _ui_scene_node_2) "0.250000,0.250000,0.250000"))
      (Variables|Default|SetRight_UI (Math|Transform|MakeTransform (Math|Vector|MakeVector (.x _returnvalue) (- (.y _returnvalue) 1e+02) (.z _returnvalue)) (Transformation|GetWorldRotation _ui_scene_node) "0.250000,0.250000,0.250000"))
      (CallFunction|SpawnUI))
    (:then_1
      (bind _returnvalue_4 (Rendering|Material|CreateDynamicMaterialInstance "/Game/AllMallsAreWalls/VisualEffects/Materials/MAT_CelShader_Inst.MAT_CelShader_Inst" "None" "None" :!class /Script/Engine.KismetMaterialLibrary))
      (bind _output_get (Variables|Default|SetMatInstRefCel _returnvalue_4))
      (bind _returnvalue_5 (Rendering|Material|CreateDynamicMaterialInstance "/Game/AllMallsAreWalls/VisualEffects/Materials/MAT_RetroOverlay_Inst.MAT_RetroOverlay_Inst" "None" "None" :!class /Script/Engine.KismetMaterialLibrary))
      (bind _output_get_2 (Variables|Default|SetMatInstRefOverlay _returnvalue_5))
      (Variables|/Script/Engine.PostProcessVolume|SetSettings (Variables|Default|GetPostProcessVolumeReference) (Utilities|Struct|MakePostProcessSettings (Utilities|Struct|MakeWeightedBlendables (Utilities|Array|MakeArray (Utilities|Struct|MakeWeightedBlendable 1.0 _output_get_2) (Utilities|Struct|MakeWeightedBlendable 1.0 _output_get))))))))

(event Input|ActionEvents|InputActionBasic_Attack
  (params (Key :type Key%20Structure :default "None"))
  (:Pressed
    ;[1 1 1] PurseSwing
    (Development|SetHiddeninGame (Variables|Default|Getgun) true false)
    (Development|SetHiddeninGame (Variables|Default|GetPurse) false false)
    (Game|SpawnActorfromClass "/Game/AllMallsAreWalls/Core/CharacterBlueprints/Purse_Melee.Purse_Melee_C" (Transformation|GetWorldTransform (Variables|Default|GetArrow1)) "Undefined" 0 0)))

(event Input|ActionEvents|InputActionshoppingcart
  (params (Key :type Key%20Structure :default "None"))
  (bind _charactermovement (Variables|Character|GetCharacterMovement))
  (bind _charactermovement_2 (Variables|Character|GetCharacterMovement))
  (:Pressed
    ;[1 1 1] Cart Ride
    (if (<= (Variables|Default|Getcart%20cooldown) 0.0)
      (if (Variables|Default|GetCartUnlock)
        (bind _output_get (Variables|Default|Setis_pressed true))
        (if _output_get
          (Development|SetHiddeninGame (Variables|Default|Getshoppingcart) false false)
          (Development|SetHiddeninGame (Variables|Default|GetPurse) true false)
          (Development|SetHiddeninGame (Variables|Default|Getgun) true false)
          (Variables|/Script/Engine.CharacterMovementComponent|SetMaxWalkSpeed _charactermovement (+ (Variables|/Script/Engine.CharacterMovementComponent|GetMaxWalkSpeed _charactermovement) 2e+04))))))
  (:Released
    (if (Variables|Default|Getis_pressed)
      (Variables|/Script/Engine.CharacterMovementComponent|SetMaxWalkSpeed _charactermovement_2 (- (Variables|/Script/Engine.CharacterMovementComponent|GetMaxWalkSpeed _charactermovement_2) 2e+04))
      (Development|SetHiddeninGame (Variables|Default|Getshoppingcart) true false)
      (Development|SetHiddeninGame (Variables|Default|GetPurse) false false)
      (Game|SpawnActorfromClass "/Game/AllMallsAreWalls/Core/CharacterBlueprints/BP_ShoppingCart.BP_ShoppingCart_C" (Transformation|GetWorldTransform (Variables|Default|GetArrow1)) "Undefined" 0 0)
      (Variables|Default|Setcart%20cooldown 6.0)
      (Variables|Default|Setis_pressed false))))

(event Input|ActionEvents|InputActionGrenade
  (params (Key :type Key%20Structure :default "None"))
  (bind _scene1 (Variables|Default|GetScene1))
  (bind _returnvalue (Transformation|GetWorldRotation _scene1))
  (:Pressed
    ;[1 1 1] Grenade Throw
    (if (<= (Variables|Default|Getdrink%20cooldown) 0.0)
      (if (Variables|Default|GetDrinkUnlock)
        (bind _returnvalue_2 (Game|SpawnActorfromClass "/Game/AllMallsAreWalls/Core/CharacterBlueprints/Drink_Grenade.Drink_Grenade_C" (Math|Transform|MakeTransform (Transformation|GetWorldLocation (Variables|Default|GetScene)) _returnvalue "1,1,1") "Undefined" 0 0))
        (Physics|SetPhysicsLinearVelocity (Variables|/Game/AllMallsAreWalls/Core/CharacterBlueprints/Drink_Grenade.Drink_Grenade_C|GetStaticMesh _returnvalue_2) (* (Math|Vector|GetForwardVector _returnvalue) 1e+03) false "None")
        (Variables|Default|Setdrink%20cooldown 7.0)))))

(event Input|ActionEvents|InputActionProjectile
  (params (Key :type Key%20Structure :default "None"))
  (bind _scene1 (Variables|Default|GetScene1))
  (bind _returnvalue (Transformation|GetWorldLocation _scene1))
  ;[1 1 1] Projectile shot
  (:Pressed
    (if (<= (Variables|Default|Getprojectile%20cooldown) 0.0)
      (if (Variables|Default|GetHitscanUnlock)
        (Development|SetHiddeninGame (Variables|Default|Getgun) false false)
        (Development|SetHiddeninGame (Variables|Default|GetPurse) true false)
        (bind _outhit (Collision|LineTraceByChannel _returnvalue (+ _returnvalue (* (Math|Vector|GetForwardVector (Transformation|GetWorldRotation _scene1)) 4e+03)) "TraceTypeQuery1" false 0 "ForDuration"))
        (Utilities|FlowControl|Sequence
          (:then_0
            (bind _asnpc_shopee (Utilities|Casting|CastToNPC_SHOPEE (.HitActor (Collision|BreakHitResult _outhit))))
            (Default|TakeDamage _asnpc_shopee 1e+02))
          (:then_1
            (bind _asnpc_scene_kids (Utilities|Casting|CastToNPC_SceneKids (.HitActor (Collision|BreakHitResult _outhit))))
            (Default|TakeDamage _asnpc_scene_kids 1e+02))
          (:then_2
            (bind _asnpc_mall_rats (Utilities|Casting|CastToNPC_MallRats (.HitActor (Collision|BreakHitResult _outhit))))
            (Default|TakeDamage _asnpc_mall_rats 1e+02))
          (:then_3
            (bind _asnpc_vsco_girl (Utilities|Casting|CastToNPC_VSCO_Girl (.HitActor (Collision|BreakHitResult _outhit))))
            (Default|TakeDamage _asnpc_vsco_girl 1e+02)))
        (Class|AISenseDamage|ReportDamageEvent (.HitActor (Collision|BreakHitResult _outhit)) self 0.0 (Transformation|GetWorldLocation (Variables|Default|GetCapsuleComponent)))
        (Variables|Default|Setprojectile%20cooldown 2.0)))))

(event Input|KeyboardEvents|M
  (params (Key :type Key%20Structure :default "None"))
  (:Pressed
    (Development|ExecuteConsoleCommand "RestartLevel" 0)))

(fn ConstructionScript)

(fn TakeDamage
  (bind _abilities (Variables|Default|GetAbilities))
  (if (> (Utilities|Array|Length _abilities) 0)
    (switch int (Utilities|Array|Get(acopy) _abilities) ; 0 - drink; 1 - cart; 2- hitscan
      (:0
        (Variables|Default|SetDrinkUnlock false))
      (:1
        (Variables|Default|SetCartUnlock false))
      (:2
        (Variables|Default|SetHitscanUnlock false)))
    (Utilities|Array|RemoveIndex _abilities)
    (Development|SetHiddeninGame (Variables|/Script/Engine.Actor|GetRootComponent (Variables|Default|GetLeft_Cup)) true true)
    (CallFunction|UpdateUI)
    (CallFunction|UpdateShaders)
    (else
      (Variables|Default|SetAmDead true))))

(fn Addability
  (params (ability :type Integer))
  (Utilities|Array|Add (Variables|Default|GetAbilities) ability)
  (CallFunction|UpdateUI)
  (CallFunction|UpdateShaders))

(fn UpdateUI
  (for (_array_element _array_index) (Variables|Default|GetAbilities)
    (Variables|Default|SetArray%20Element _array_element)
    (switch int _array_index
      (:0
        (Utilities|FlowControl|DoOnce false
          (:Completed
            (Development|PrintString "right")
            (switch int (Variables|Default|GetArray%20Element)
              (:0
                (Development|SetHiddeninGame (Variables|/Script/Engine.Actor|GetRootComponent (Variables|Default|GetRight_Cup)) false true))
              (:1
                (Development|SetHiddeninGame (Variables|/Script/Engine.Actor|GetRootComponent (Variables|Default|GetRight_ShoppingCart)) false true))
              (:2
                (Development|SetHiddeninGame (Variables|/Script/Engine.Actor|GetRootComponent (Variables|Default|GetRight_Peircing)) false true))))))
      (:1
        (Utilities|FlowControl|DoOnce false
          (:Completed
            (Development|PrintString "Middle")
            (switch int (Variables|Default|GetArray%20Element)
              (:0
                (Development|SetHiddeninGame (Variables|/Script/Engine.Actor|GetRootComponent (Variables|Default|GetMiddle_Cup)) false true))
              (:1
                (Development|SetHiddeninGame (Variables|/Script/Engine.Actor|GetRootComponent (Variables|Default|GetMiddle_SHoppingCart)) false true))
              (:2
                (Development|SetHiddeninGame (Variables|/Script/Engine.Actor|GetRootComponent (Variables|Default|GetMiddle_Peirce)) false true))))))
      (:2
        (Utilities|FlowControl|DoOnce false
          (:Completed
            (Development|PrintString "left")
            (switch int (Variables|Default|GetArray%20Element)
              (:0
                (Development|SetHiddeninGame (Variables|/Script/Engine.Actor|GetRootComponent (Variables|Default|GetLeft_Cup)) false true))
              (:1
                (Development|SetHiddeninGame (Variables|/Script/Engine.Actor|GetRootComponent (Variables|Default|GetLeftt_ShoppingCart)) false true))
              (:2
                (Development|SetHiddeninGame (Variables|/Script/Engine.Actor|GetRootComponent (Variables|Default|Getleft_Peirce)) false true)))))))))

(fn SpawnUI
  (bind _returnvalue (Game|SpawnActorfromClass "/Game/AllMallsAreWalls/Core/CharacterBlueprints/Rotators/Cup.Cup_C" (Variables|Default|GetRight_UI) "AlwaysSpawn" 0 0))
  (bind _output_get (Variables|Default|SetRight_Cup _returnvalue))
  (Development|SetHiddeninGame (Variables|/Script/Engine.Actor|GetRootComponent _output_get) true true)
  (Transformation|AttachComponentToComponent _output_get (Variables|Default|GetUI_Right_Scene) "None" "SnapToTarget" "KeepRelative" "SnapToTarget" false)
  (bind _returnvalue_2 (Game|SpawnActorfromClass "/Game/AllMallsAreWalls/Core/CharacterBlueprints/Rotators/SMOLSHOPPINGCART.SMOLSHOPPINGCART_C" (Variables|Default|GetRight_UI) "AlwaysSpawn" 0 0))
  (bind _output_get_2 (Variables|Default|SetRight_ShoppingCart _returnvalue_2))
  (Development|SetHiddeninGame (Variables|/Script/Engine.Actor|GetRootComponent _output_get_2) true true)
  (Transformation|AttachComponentToComponent _output_get_2 (Variables|Default|GetUI_Right_Scene) "None" "SnapToTarget" "KeepRelative" "SnapToTarget" false)
  (bind _returnvalue_3 (Game|SpawnActorfromClass "/Game/AllMallsAreWalls/Core/CharacterBlueprints/Rotators/Peircing_Gun.Peircing_Gun_C" (Variables|Default|GetRight_UI) "AlwaysSpawn" 0 0))
  (bind _output_get_3 (Variables|Default|SetRight_Peircing _returnvalue_3))
  (Development|SetHiddeninGame (Variables|/Script/Engine.Actor|GetRootComponent _output_get_3) true true)
  (Transformation|AttachComponentToComponent _output_get_3 (Variables|Default|GetUI_Right_Scene) "None" "SnapToTarget" "KeepRelative" "SnapToTarget" false)
  (bind _returnvalue_4 (Game|SpawnActorfromClass "/Game/AllMallsAreWalls/Core/CharacterBlueprints/Rotators/Cup.Cup_C" (Variables|Default|GetMiddle_UI) "AlwaysSpawn" 0 0))
  (bind _output_get_4 (Variables|Default|SetMiddle_Cup _returnvalue_4))
  (Development|SetHiddeninGame (Variables|/Script/Engine.Actor|GetRootComponent _output_get_4) true true)
  (Transformation|AttachComponentToComponent _output_get_4 (Variables|Default|GetUI_Scene_Node) "None" "SnapToTarget" "KeepRelative" "SnapToTarget" false)
  (bind _returnvalue_5 (Game|SpawnActorfromClass "/Game/AllMallsAreWalls/Core/CharacterBlueprints/Rotators/SMOLSHOPPINGCART.SMOLSHOPPINGCART_C" (Variables|Default|GetMiddle_UI) "AlwaysSpawn" 0 0))
  (bind _output_get_5 (Variables|Default|SetMiddle_SHoppingCart _returnvalue_5))
  (Development|SetHiddeninGame (Variables|/Script/Engine.Actor|GetRootComponent _output_get_5) true true)
  (Transformation|AttachComponentToComponent _output_get_5 (Variables|Default|GetUI_Scene_Node) "None" "SnapToTarget" "KeepRelative" "SnapToTarget" false)
  (bind _returnvalue_6 (Game|SpawnActorfromClass "/Game/AllMallsAreWalls/Core/CharacterBlueprints/Rotators/Peircing_Gun.Peircing_Gun_C" (Variables|Default|GetMiddle_UI) "AlwaysSpawn" 0 0))
  (bind _output_get_6 (Variables|Default|SetMiddle_Peirce _returnvalue_6))
  (Development|SetHiddeninGame (Variables|/Script/Engine.Actor|GetRootComponent _output_get_6) true true)
  (Transformation|AttachComponentToComponent _output_get_6 (Variables|Default|GetUI_Scene_Node) "None" "SnapToTarget" "KeepRelative" "SnapToTarget" false)
  (bind _returnvalue_7 (Game|SpawnActorfromClass "/Game/AllMallsAreWalls/Core/CharacterBlueprints/Rotators/Cup.Cup_C" (Variables|Default|GetLeft_UI) "AlwaysSpawn" 0 0))
  (bind _output_get_7 (Variables|Default|SetLeft_Cup _returnvalue_7))
  (Development|SetHiddeninGame (Variables|/Script/Engine.Actor|GetRootComponent _output_get_7) true true)
  (Transformation|AttachComponentToComponent _output_get_7 (Variables|Default|GetUI_Left_Scene) "None" "SnapToTarget" "KeepRelative" "SnapToTarget" false)
  (bind _returnvalue_8 (Game|SpawnActorfromClass "/Game/AllMallsAreWalls/Core/CharacterBlueprints/Rotators/SMOLSHOPPINGCART.SMOLSHOPPINGCART_C" (Variables|Default|GetLeft_UI) "AlwaysSpawn" 0 0))
  (bind _output_get_8 (Variables|Default|SetLeftt_ShoppingCart _returnvalue_8))
  (Development|SetHiddeninGame (Variables|/Script/Engine.Actor|GetRootComponent _output_get_8) true true)
  (Transformation|AttachComponentToComponent _output_get_8 (Variables|Default|GetUI_Left_Scene) "None" "SnapToTarget" "KeepRelative" "SnapToTarget" false)
  (bind _returnvalue_9 (Game|SpawnActorfromClass "/Game/AllMallsAreWalls/Core/CharacterBlueprints/Rotators/Peircing_Gun.Peircing_Gun_C" (Variables|Default|GetLeft_UI) "AlwaysSpawn" 0 0))
  (bind _output_get_9 (Variables|Default|Setleft_Peirce _returnvalue_9))
  (Development|SetHiddeninGame (Variables|/Game/AllMallsAreWalls/Core/CharacterBlueprints/Rotators/Peircing_Gun.Peircing_Gun_C|GetStaticMesh _output_get_9) true true)
  (Transformation|AttachComponentToComponent _output_get_9 (Variables|Default|GetUI_Left_Scene) "None" "SnapToTarget" "KeepRelative" "SnapToTarget" false))

(fn UpdateTransparenctUI
  (params (DrinkCD :type Float%20%28single-precision%29) (ProjCD :type Float%20%28single-precision%29) (CartCD :type Float%20%28single-precision%29))
  (bind _returnvalue (/ DrinkCD 7.0))
  (bind _returnvalue_2 (/ CartCD 6.0))
  (bind _returnvalue_3 (/ ProjCD 2.0))
  (bind _returnvalue_4 (- 1.0 _returnvalue))
  (bind _returnvalue_5 (- 1.0 _returnvalue_2))
  (bind _returnvalue_6 (- 1.0 _returnvalue_3))
  (Utilities|FlowControl|Sequence
    (:then_0
      (if (<= _returnvalue 0.0)
        (Default|SetTransparency (Variables|Default|GetRight_Cup) 1.0)
        (Default|SetTransparency (Variables|Default|GetMiddle_Cup) 1.0)
        (Default|SetTransparency (Variables|Default|GetLeft_Cup) 1.0)
        (else
          (Default|SetTransparency (Variables|Default|GetRight_Cup) _returnvalue_4)
          (Default|SetTransparency (Variables|Default|GetMiddle_Cup) _returnvalue_4)
          (Default|SetTransparency (Variables|Default|GetLeft_Cup) _returnvalue_4))))
    (:then_1
      (if (<= _returnvalue_3 0.0)
        (Default|SetTransparency (Variables|Default|GetRight_Peircing) 1.0)
        (Default|SetTransparency (Variables|Default|GetMiddle_Peirce) 1.0)
        (Default|SetTransparency (Variables|Default|Getleft_Peirce) 1.0)
        (else
          (Default|SetTransparency (Variables|Default|GetRight_Peircing) _returnvalue_6)
          (Default|SetTransparency (Variables|Default|GetMiddle_Peirce) _returnvalue_6)
          (Default|SetTransparency (Variables|Default|Getleft_Peirce) _returnvalue_6))))
    (:then_2
      (if (<= _returnvalue_2 0.0)
        (Default|SetTransparency (Variables|Default|GetRight_ShoppingCart) 1.0)
        (Default|SetTransparency (Variables|Default|GetMiddle_SHoppingCart) 1.0)
        (Default|SetTransparency (Variables|Default|GetLeftt_ShoppingCart) 1.0)
        (else
          (Default|SetTransparency (Variables|Default|GetRight_ShoppingCart) _returnvalue_5)
          (Default|SetTransparency (Variables|Default|GetMiddle_SHoppingCart) _returnvalue_5)
          (Default|SetTransparency (Variables|Default|GetLeftt_ShoppingCart) _returnvalue_5))))))

(fn UpdateShaders
  (bind _0hpsettings (Variables|Default|Get0HPSettings))
  (bind _2hpsettings (Variables|Default|Get2HPSettings))
  (bind _1hpsettings (Variables|Default|Get1HPSettings))
  (switch int (Utilities|Array|Length (Variables|Default|GetAbilities))
    (:0
      (Rendering|Material|SetScalarParameterValue (Variables|Default|GetMatInstRefOverlay) "Bar Intensity" (Utilities|Array|Get(acopy) _0hpsettings) :!class /Script/Engine.MaterialInstanceDynamic)
      (Rendering|Material|SetScalarParameterValue (Variables|Default|GetMatInstRefOverlay) "Brightness" (Utilities|Array|Get(acopy) _0hpsettings 1) :!class /Script/Engine.MaterialInstanceDynamic)
      (Rendering|Material|SetScalarParameterValue (Variables|Default|GetMatInstRefOverlay) "Desaturation" (Utilities|Array|Get(acopy) _0hpsettings 2) :!class /Script/Engine.MaterialInstanceDynamic)
      (Rendering|Material|SetScalarParameterValue (Variables|Default|GetMatInstRefOverlay) "Distortion Bar Size" (Utilities|Array|Get(acopy) _0hpsettings 3) :!class /Script/Engine.MaterialInstanceDynamic)
      (Rendering|Material|SetScalarParameterValue (Variables|Default|GetMatInstRefOverlay) "Hertz" (Utilities|Array|Get(acopy) _0hpsettings 4) :!class /Script/Engine.MaterialInstanceDynamic)
      (Rendering|Material|SetScalarParameterValue (Variables|Default|GetMatInstRefOverlay) "Noise Strength" (Utilities|Array|Get(acopy) _0hpsettings 5) :!class /Script/Engine.MaterialInstanceDynamic)
      (Rendering|Material|SetVectorParameterValue (Variables|Default|GetMatInstRefOverlay) "Bar Speed" (Math|Conversions|ToLinearColor(Vector) (Math|Vector|MakeVector 0.0 (Utilities|Array|Get(acopy) _0hpsettings 6) 0.0)) :!class /Script/Engine.MaterialInstanceDynamic))
    (:1
      (Rendering|Material|SetScalarParameterValue (Variables|Default|GetMatInstRefOverlay) "Bar Intensity" (Utilities|Array|Get(acopy) _1hpsettings) :!class /Script/Engine.MaterialInstanceDynamic)
      (Rendering|Material|SetScalarParameterValue (Variables|Default|GetMatInstRefOverlay) "Brightness" (Utilities|Array|Get(acopy) _1hpsettings 1) :!class /Script/Engine.MaterialInstanceDynamic)
      (Rendering|Material|SetScalarParameterValue (Variables|Default|GetMatInstRefOverlay) "Desaturation" (Utilities|Array|Get(acopy) _1hpsettings 2) :!class /Script/Engine.MaterialInstanceDynamic)
      (Rendering|Material|SetScalarParameterValue (Variables|Default|GetMatInstRefOverlay) "Distortion Bar Size" (Utilities|Array|Get(acopy) _1hpsettings 3) :!class /Script/Engine.MaterialInstanceDynamic)
      (Rendering|Material|SetScalarParameterValue (Variables|Default|GetMatInstRefOverlay) "Hertz" (Utilities|Array|Get(acopy) _1hpsettings 4) :!class /Script/Engine.MaterialInstanceDynamic)
      (Rendering|Material|SetScalarParameterValue (Variables|Default|GetMatInstRefOverlay) "Noise Strength" (Utilities|Array|Get(acopy) _1hpsettings 5) :!class /Script/Engine.MaterialInstanceDynamic)
      (Rendering|Material|SetVectorParameterValue (Variables|Default|GetMatInstRefOverlay) "Bar Speed" (Math|Conversions|ToLinearColor(Vector) (Math|Vector|MakeVector 0.0 (Utilities|Array|Get(acopy) _1hpsettings 6) 0.0)) :!class /Script/Engine.MaterialInstanceDynamic))
    (:2
      (Rendering|Material|SetScalarParameterValue (Variables|Default|GetMatInstRefOverlay) "Bar Intensity" (Utilities|Array|Get(acopy) _2hpsettings) :!class /Script/Engine.MaterialInstanceDynamic)
      (Rendering|Material|SetScalarParameterValue (Variables|Default|GetMatInstRefOverlay) "Brightness" (Utilities|Array|Get(acopy) _2hpsettings 1) :!class /Script/Engine.MaterialInstanceDynamic)
      (Rendering|Material|SetScalarParameterValue (Variables|Default|GetMatInstRefOverlay) "Desaturation" (Utilities|Array|Get(acopy) _2hpsettings 2) :!class /Script/Engine.MaterialInstanceDynamic)
      (Rendering|Material|SetScalarParameterValue (Variables|Default|GetMatInstRefOverlay) "Distortion Bar Size" (Utilities|Array|Get(acopy) _2hpsettings 3) :!class /Script/Engine.MaterialInstanceDynamic)
      (Rendering|Material|SetScalarParameterValue (Variables|Default|GetMatInstRefOverlay) "Hertz" (Utilities|Array|Get(acopy) _2hpsettings 4) :!class /Script/Engine.MaterialInstanceDynamic)
      (Rendering|Material|SetScalarParameterValue (Variables|Default|GetMatInstRefOverlay) "Noise Strength" (Utilities|Array|Get(acopy) _2hpsettings 5) :!class /Script/Engine.MaterialInstanceDynamic)
      (Rendering|Material|SetVectorParameterValue (Variables|Default|GetMatInstRefOverlay) "Bar Speed" (Math|Conversions|ToLinearColor(Vector) (Math|Vector|MakeVector 0.0 (Utilities|Array|Get(acopy) _2hpsettings 6) 0.0)) :!class /Script/Engine.MaterialInstanceDynamic))
    (:3
      (Rendering|Material|SetScalarParameterValue (Variables|Default|GetMatInstRefOverlay) "Bar Intensity" (Utilities|Array|Get(acopy) (Variables|Default|GetFullHPSettings)) :!class /Script/Engine.MaterialInstanceDynamic)
      (Rendering|Material|SetScalarParameterValue (Variables|Default|GetMatInstRefOverlay) "Brightness" (Utilities|Array|Get(acopy) (Variables|Default|GetFullHPSettings) 1) :!class /Script/Engine.MaterialInstanceDynamic)
      (Rendering|Material|SetScalarParameterValue (Variables|Default|GetMatInstRefOverlay) "Desaturation" (Utilities|Array|Get(acopy) (Variables|Default|GetFullHPSettings) 2) :!class /Script/Engine.MaterialInstanceDynamic)
      (Rendering|Material|SetScalarParameterValue (Variables|Default|GetMatInstRefOverlay) "Distortion Bar Size" (Utilities|Array|Get(acopy) (Variables|Default|GetFullHPSettings) 3) :!class /Script/Engine.MaterialInstanceDynamic)
      (Rendering|Material|SetScalarParameterValue (Variables|Default|GetMatInstRefOverlay) "Hertz" (Utilities|Array|Get(acopy) (Variables|Default|GetFullHPSettings) 4) :!class /Script/Engine.MaterialInstanceDynamic)
      (Rendering|Material|SetScalarParameterValue (Variables|Default|GetMatInstRefOverlay) "Noise Strength" (Utilities|Array|Get(acopy) (Variables|Default|GetFullHPSettings) 5) :!class /Script/Engine.MaterialInstanceDynamic)
      (Rendering|Material|SetVectorParameterValue (Variables|Default|GetMatInstRefOverlay) "Bar Speed" (Math|Conversions|ToLinearColor(Vector) (Math|Vector|MakeVector 0.0 (Utilities|Array|Get(acopy) (Variables|Default|GetFullHPSettings) 6) 0.0)) :!class /Script/Engine.MaterialInstanceDynamic))))