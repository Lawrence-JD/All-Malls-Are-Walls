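; BP_ShoppingCart is a shopping cart actor that damages mall NPCs when its static mesh hits them.
; On hit, a sequence tries four casts (Shopee, Scene Kids, Mall Rats, VSCO Girl) and applies the same fixed damage to a match.
; It then reports an AI damage-sense event naming player pawn 0 as instigator, located at the player's capsule rather than the impact point.
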(event OnComponentHit(StaticMesh)
  (params (HitComponent :type Primitive%20Component%20Object%20Reference) (OtherActor :type Actor%20Object%20Reference) (OtherComp :type Primitive%20Component%20Object%20Reference) (NormalImpulse :type Vector :default "0, 0, 0") (Hit :type Hit%20Result%20Structure%20%28by%20ref%29))
  (Utilities|FlowControl|Sequence
    (:then_0
      (bind _asnpc_shopee (Utilities|Casting|CastToNPC_SHOPEE OtherActor))
      (Default|TakeDamage _asnpc_shopee 1e+02))
    (:then_1
      (bind _asnpc_scene_kids (Utilities|Casting|CastToNPC_SceneKids OtherActor))
      (Default|TakeDamage _asnpc_scene_kids 1e+02))
    (:then_2
      (bind _asnpc_mall_rats (Utilities|Casting|CastToNPC_MallRats OtherActor))
      (Default|TakeDamage _asnpc_mall_rats 1e+02))
    (:then_3
      (bind _asnpc_vsco_girl (Utilities|Casting|CastToNPC_VSCO_Girl OtherActor))
      (Default|TakeDamage _asnpc_vsco_girl 1e+02)))
  (bind _asbp_player_character (Utilities|Casting|CastToBP_PlayerCharacter (Game|Player|GetPlayerPawn 0)))
  (Class|AISenseDamage|ReportDamageEvent OtherActor _asbp_player_character 0.0 (Transformation|GetWorldLocation (Variables|/Script/Engine.Character|GetCapsuleComponent _asbp_player_character))))

(event EventBeginPlay)

(event Collision|EventActorBeginOverlap
  (params (OtherActor :type Actor%20Object%20Reference)))

(event EventTick
  (params (DeltaSeconds :type Float%20%28single-precision%29)))

(fn ConstructionScript)